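; BP_AK_enemy is an AK-105 rifle Blueprint, named for enemy use, that handles firing, ammo and reloading.
; Shooting spawns BP_Bullet at ArrowFire, decrements Ammo and adds muzzle effects, sound and camera shake, or only plays a sound when empty.
; It also runs a line trace whose result is unused and makes noise with the player character as instigator.
; Reloading refills Ammo toward 30 from the FullMagazine reserve.
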(event `AmmoCounter`
  (if (stale `self.Shooting` IsShooting)
    (set `self.Ammo` (- (`self.Ammo`) 1))))

(event `self.Shooting`
  (params (IsShooting :type Boolean))
  (bind _arrowfire (`self.ArrowFire`))
  (bind _returnvalue (`SceneComponent.K2_GetComponentLocation` _arrowfire))
  (bind (_returnvalue_location _returnvalue_rotation) (`KismetMathLibrary.BreakTransform` (`SceneComponent.K2_GetComponentToWorld` (`self.ArrowFire`))))
  (if (<= (`self.Ammo`) 0)
    (`GameplayStatics.SpawnSound2D` null 1.0 1.0 0.0 null)
    (elif IsShooting
      (bind _returnvalue_2 (`|SpawnActorFromClass` "/Game/Weapon/AK105/BP_Bullet.BP_Bullet_C" (`KismetMathLibrary.MakeTransform` _returnvalue_location _returnvalue_rotation) "Undefined" "MultiplyWithRoot" null null))
      (`KismetSystemLibrary.LineTraceSingle` _returnvalue (+ _returnvalue (* (`KismetMathLibrary.GetForwardVector` (`SceneComponent.K2_GetComponentRotation` _arrowfire)) 4000.0)) "TraceTypeQuery2" false (`|MakeArray` _returnvalue_2 :!type "Actor Object Reference"))
      (`self.AmmoCounter`)
      (`AddComponent|NODE_AddCameraShakeSourceComponent-0`)
      (`NiagaraFunctionLibrary.SpawnSystemAttached` "/Game/MixedVFX/Particles/Projectiles/NS_Projectile_01.NS_Projectile_01" (`self.ArrowFire`) "None" (0.0 0.0 0.0) (struct) "SnapToTargetIncludingScale")
      (`GameplayStatics.SpawnSound2D` "/Game/StarterContent/Audio/Explosion01.Explosion01" 0.01 1.0 15.0 null)
      (`self.MakeNoise` 1.0 (`GameplayStatics.GetPlayerCharacter` 0) (`self.K2_GetActorLocation`) 3000.0 "Noise"))))

(event `self.Reloading`
  (params (BIsReloading :type Boolean) (ReloadTime :type "Float (double-precision)"))
  (bind _fullmagazine (`self.FullMagazine`))
  (if BIsReloading
    (set `self.CommonAmmo` _fullmagazine)
    (set `self.FullMagazine` (`KismetMathLibrary.Clamp` (- _fullmagazine (- 30 (`self.Ammo`))) 0 _fullmagazine))
    (set `self.Ammo` (+ (- (`self.CommonAmmo`) (`self.FullMagazine`)) (`self.Ammo`)))))

(fn `UserConstructionScript`)